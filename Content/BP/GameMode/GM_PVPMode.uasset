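; GM_PVPMode is the game mode for PVP matches, starting the game once enough players have joined.
; On BeginPlay it caches the game state as BP_WildGameState.
; After each login and a short delay, it adds the BP_WildPlayerController to the game state's Players array, then calls StartGame on that state when at least two players are present.
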(event EventBeginPlay
  (bind _asbp_wild_game_state (Utilities|Casting|CastToBP_WildGameState (Game|GetGameState)))
  (Variables|Default|SetWildGameState _asbp_wild_game_state))

(event EventTick
  (params (DeltaSeconds :type Float%20%28single-precision%29)))

(event EventPostLogin
  (params (NewPlayer :type Player%20Controller%20Object%20Reference))
  (Development|PrintText "OnPostLogin")
  (Utilities|FlowControl|Delay 0.1)
  (bind _asbp_wild_player_controller (Utilities|Casting|CastToBP_WildPlayerController NewPlayer))
  (Utilities|Array|Add (Variables|/Game/BP/GameSate/BP_WildGameState.BP_WildGameState_C|GetPlayers (Variables|Default|GetWildGameState)) _asbp_wild_player_controller)
  (bind _returnvalue (Class|GameModeBase|GetNumPlayers))
  (if (>= _returnvalue 2)
    (Default|StartGame (Variables|Default|GetWildGameState))))

(fn ConstructionScript)