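; BP_WildGameState is a game state that tracks the current player and drives the game through phase objects.
; On BeginPlay it spawns the game-set phase actor from a configurable class and initializes it with a reference to itself.
; StartGame makes the first entry in Players the current player, then calls SetPhase, which stores that phase as current and starts it.
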(event Custom|StartGame
  (Variables|Default|SetCurrentPlayer (Utilities|Array|Get(acopy) (Variables|Default|GetPlayers)))
  (Development|PrintText "Start Game")
  (CallFunction|SetPhase (Variables|Default|GetGameSetPhase)))

(event EventBeginPlay
  (bind _returnvalue (Game|SpawnActorfromClass (Variables|Default|GetGameSetPhaseClass) (Math|Transform|MakeTransform "0, 0, 0") "Undefined" "MultiplyWithRoot" 0 0))
  (Class|WildGamePhaseBase|InitPhase _returnvalue self)
  (Variables|Default|SetGameSetPhase _returnvalue))

(event EventTick
  (params (DeltaSeconds :type Float%20%28single-precision%29)))

(fn ConstructionScript)

(fn SetPhase
  (params (Phase :type Wild%20Game%20Phase%20Base%20Object%20Reference))
  (bind _output_get (Variables|Default|SetCurrentPhase Phase))
  (Class|WildGamePhaseBase|StartPhase _output_get))